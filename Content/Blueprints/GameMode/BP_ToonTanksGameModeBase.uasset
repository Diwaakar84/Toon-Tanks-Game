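; Game mode Blueprint for Toon Tanks that shows the start and end-of-game screens.
; GameStart creates the start widget and adds it to the viewport.
; GameOver creates the end-game widget, sets its text to a green win or red loss message from the WonGame flag, then displays it.
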(event EventBeginPlay)

(event EventTick
  (params (DeltaSeconds :type Float%20%28single-precision%29)))

(event EventGameStart
  (bind _returnvalue (UserInterface|CreateWidget "/Game/Blueprints/Widget/WBP_StartGameWidget.WBP_StartGameWidget_C"))
  (UserInterface|Viewport|AddtoViewport _returnvalue 0))

(event EventGameOver
  (params (bWonGame :type Boolean))
  (bind _returnvalue (UserInterface|CreateWidget "/Game/Blueprints/Widget/WBP_EndGameWidget.WBP_EndGameWidget_C"))
  (if bWonGame
    (Rendering|Components|TextRender|SetText (Variables|/Game/Blueprints/Widget/WBP_EndGameWidget.WBP_EndGameWidget_C|GetDisplayText _returnvalue) "You Won!!!")
    (Appearance|SetColorandOpacity (Variables|/Game/Blueprints/Widget/WBP_EndGameWidget.WBP_EndGameWidget_C|GetDisplayText _returnvalue) (Utilities|Struct|MakeSlateColor "(R=0.018742,G=1.000000,B=0.000000,A=1.000000)") :!class /Script/UMG.TextBlock)
    (else
      (Rendering|Components|TextRender|SetText (Variables|/Game/Blueprints/Widget/WBP_EndGameWidget.WBP_EndGameWidget_C|GetDisplayText _returnvalue) "You Lost!!!")
      (Appearance|SetColorandOpacity (Variables|/Game/Blueprints/Widget/WBP_EndGameWidget.WBP_EndGameWidget_C|GetDisplayText _returnvalue) (Utilities|Struct|MakeSlateColor "(R=1.000000,G=0.000000,B=0.007639,A=1.000000)") :!class /Script/UMG.TextBlock)))
  (UserInterface|Viewport|AddtoViewport _returnvalue 0))

(fn ConstructionScript)